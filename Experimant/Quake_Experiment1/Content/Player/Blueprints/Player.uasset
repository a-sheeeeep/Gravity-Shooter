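; Player character with Source-style first-person movement, auto bunny hopping and gravity that follows the surface beneath it.
; Tick applies yaw, then runs ground friction and acceleration or capped air acceleration, all pushed through AddMovementInput rather than setting velocity.
; Orientation traces down and along velocity, eases the actor's up vector toward the hit normal and points gravity opposite it.
; Holding Jump re-jumps after landing; pitch rotates the camera within clamped limits.
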(event `InputAxis|Turn`
  (params (AxisValue :type "Float (single-precision)"))
  (set `self.Camera_Turn` (* AxisValue (`self.sens`))))

(event `self.ReceiveBeginPlay`
  (set `self.accel_const` 10.0)
  (set `self.wishspeed` 600.0)
  (set `self.Friction Const` 2.0)
  (set `self.sens` 50.0))

(event `InputAxis|Forward`
  (params (AxisValue :type "Float (single-precision)")))

(event `self.ReceiveActorBeginOverlap`
  (params (OtherActor :type "Actor Object Reference")))

(event `InputAxis|Right`
  (params (AxisValue :type "Float (single-precision)")))

(event `self.ReceiveTick`
  (params (DeltaSeconds :type "Float (single-precision)"))
  (`self.K2_AddActorLocalRotation` (`KismetMathLibrary.MakeRotator` 0.0 0.0 (* (`GameplayStatics.GetWorldDeltaSeconds`) (`self.Camera_Turn`))))
  (if (not (`NavMovementComponent.IsFalling` (`self.CharacterMovement`)))
    (`self.SV_Friction`)
    (`self.SV_Accelerate` (stale `InputAxis|Forward` AxisValue) (stale `InputAxis|Right` AxisValue))
    (else
      (`self.SV_AirAccelerate` (stale `InputAxis|Forward` AxisValue) (stale `InputAxis|Right` AxisValue))))
  (`self.Orientation`))

(event `InputAxis|Pitch`
  (params (AxisValue :type "Float (single-precision)"))
  (`self.Pitch` AxisValue))

(event `InputAction|Jump`
  (params (Key :type "Key Structure"))
  (:`Pressed`
    (set `self.auto_hop` true)
    (`self.Jump`))
  (:`Released`
    (set `self.auto_hop` false)))

(event `self.OnLanded`
  (params (Hit :type "HitResult Structure (by ref)"))
  (if (`self.auto_hop`)
    (`KismetSystemLibrary.Delay` 0.05)
    (`self.Jump`)))

(fn `Orientation`
  (bind _outhit (`KismetSystemLibrary.LineTraceSingle` (`self.K2_GetActorLocation`) (+ (`self.K2_GetActorLocation`) (+ (* (`self.GetActorUpVector`) -300.0) (* (`KismetMathLibrary.Normal` (`self.GetVelocity`)) 200.0))) "TraceTypeQuery1"))
  (`self.K2_SetActorRotation` (`KismetMathLibrary.MakeRotFromZX` (`KismetMathLibrary.VInterpTo` (`self.GetActorUpVector`) (`.ImpactNormal` (`GameplayStatics.BreakHitResult` _outhit)) (`GameplayStatics.GetWorldDeltaSeconds`) 10.0) (`self.GetActorForwardVector`)))
  (`CharacterMovementComponent.SetGravityDirection` (`self.CharacterMovement`) (* -1.0 (`self.GetActorUpVector`))))

(fn `Pitch`
  (params (Input :type "Float (double-precision)"))
  (set `self.Camera_Pitch` (`KismetMathLibrary.FClamp` (+ (* Input (* (`self.sens`) -1.0) (`GameplayStatics.GetWorldDeltaSeconds`)) (`self.Camera_Pitch`)) -80.0 80.0))
  (`SceneComponent.K2_SetRelativeRotation` (`self.Camera`) (`KismetMathLibrary.MakeRotator` 0.0 (`self.Camera_Pitch`)) false false))

(fn `SV_Accelerate`
  (params (X :type "Float (double-precision)") (Y :type "Float (double-precision)"))
  (set `self.WishDir` (+ (* (`self.GetActorForwardVector`) X) (* (`self.GetActorRightVector`) Y)))
  (set `self.currentspeed` (`KismetMathLibrary.Dot_VectorVector` (`self.GetVelocity`) (`self.WishDir`)))
  (set `self.add speed` (- (`self.wishspeed`) (`self.currentspeed`)))
  (if (> (`self.add speed`) 0.0)
    (set `self.accel speed` (* (`self.accel_const`) (`self.wishspeed`) (`GameplayStatics.GetWorldDeltaSeconds`)))
    (if (> (`self.accel speed`) (`self.add speed`))
      (set `self.accel speed` (`self.add speed`)))
    (set `self.Vel` (+ (`self.GetVelocity`) (* (`self.accel speed`) (`self.WishDir`))))
    (`self.AddMovementInput` (`self.WishDir`) (`self.accel speed`))))

(fn `SV_AirAccelerate`
  (params (X :type "Float (double-precision)") (Y :type "Float (double-precision)"))
  (set `self.WishDir` (+ (* X (`self.GetActorForwardVector`)) (* Y (`self.GetActorRightVector`))))
  (set `self.wishspd` (`self.wishspeed`))
  (if (> (`self.wishspd`) 60.0)
    (set `self.wishspd` 60.0))
  (set `self.currentspeed` (`KismetMathLibrary.Dot_VectorVector` (`self.WishDir`) (`self.GetVelocity`)))
  (set `self.add speed` (- (`self.wishspd`) (`self.currentspeed`)))
  (if (> (`self.add speed`) 0.0)
    (set `self.accel speed` (* (`self.accel_const`) (`self.wishspeed`) (`GameplayStatics.GetWorldDeltaSeconds`)))
    (if (> (`self.accel speed`) (`self.add speed`))
      (set `self.accel speed` (`self.add speed`)))
    (set `self.Vel` (+ (`self.Vel`) (* (`self.accel speed`) (`self.WishDir`))))
    (`self.AddMovementInput` (`self.WishDir`) (`self.accel speed`))))

(fn `SV_Friction`
  (locals (`Current Velocity` :type "Vector Structure") (`Current Speed` :type "Float (double-precision)") (`opposite direction` :type "Vector Structure") (`firction strength` :type "Float (double-precision)"))
  (bind _returnvalue (`self.GetVelocity`))
  (set `local.Current Velocity` _returnvalue)
  (set `local.Current Speed` (`KismetMathLibrary.VSize` _returnvalue))
  (if (> (`local.Current Speed`) 0.1)
    (set `local.opposite direction` (* (`KismetMathLibrary.Normal` (`local.Current Velocity`)) -1.0))
    (set `local.firction strength` (* (* (`local.Current Speed`) 0.1) (`self.Friction Const`) (`GameplayStatics.GetWorldDeltaSeconds`)))
    (`self.AddMovementInput` (`local.opposite direction`) (`local.firction strength`))))

(fn `Turn`
  (params (A :type "Float (double-precision)")))

(fn `UserConstructionScript`)