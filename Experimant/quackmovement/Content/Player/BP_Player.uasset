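; Player character with Quake/Source-style ground and air acceleration that aligns itself and its gravity to the surface underfoot.
; Each tick applies yaw locally and via a server call, sets clamped camera pitch, then feeds wish-direction acceleration, speed-capped when falling, into AddMovementInput.
; Orientation traces below and ahead along velocity, eases the up vector toward the hit normal, and points gravity opposite it.
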(event `self.ReceiveBeginPlay`
  (set `self.SV_Wishspeed` 600.0)
  (set `self.SV_Air_Accelerating` 90.0)
  (set `self.SV_accelconstant` 10.0)
  (set `self.sensitivity` 30.0))

(event `self.ReceiveTick`
  (params (DeltaSeconds :type "Float (single-precision)"))
  (bind _returnvalue (`KismetMathLibrary.MakeRotator` 0.0 0.0 (* DeltaSeconds (`self.turn_amount`))))
  (`self.K2_AddActorLocalRotation` _returnvalue)
  (`self.Server_Rotate_Yaw` _returnvalue)
  (`SceneComponent.K2_SetRelativeRotation` (`self.Camera`) (`KismetMathLibrary.MakeRotator` 0.0 (`self.pitch_amount`)) false false)
  (if (not (`NavMovementComponent.IsFalling` (`self.CharacterMovement`)))
    (`self.SV_Acceleration` (stale `InputAxis|Forward` AxisValue) (stale `InputAxis|Right` AxisValue))
    (else
      (`self.SV_AirAccelerate` (stale `InputAxis|Forward` AxisValue) (stale `InputAxis|Right` AxisValue))))
  (`self.Orientation`))

(event `InputAxis|Forward`
  (params (AxisValue :type "Float (single-precision)")))

(event `InputAxis|Right`
  (params (AxisValue :type "Float (single-precision)")))

(event `Server_Rotate_Yaw`
  (params (DeltaRotation :type "Rotator Structure"))
  (`self.K2_AddActorLocalRotation` DeltaRotation))

(event `InputAction|Jump`
  (params (Key :type "Key Structure"))
  (:`Pressed`
    (`self.Jump`)))

(event `InputAxis|Turn`
  (params (AxisValue :type "Float (single-precision)"))
  (set `self.turn_amount` (* AxisValue (`self.sensitivity`))))

(event `InputAxis|Look`
  (params (AxisValue :type "Float (single-precision)"))
  (set `self.pitch_amount` (`KismetMathLibrary.FClamp` (+ (* AxisValue (* (`self.sensitivity`) -0.01)) (`self.pitch_amount`)) -80.0 80.0)))

(fn `Friction`
  (set `self.Movement_Velocity` (* (`self.SV_Air_Accelerating`) (`self.Movement_Velocity`))))

(fn `Orientation`
  (bind _outhit (`KismetSystemLibrary.LineTraceSingle` (`self.K2_GetActorLocation`) (+ (`self.K2_GetActorLocation`) (+ (* (`self.GetActorUpVector`) -100.0) (* (`KismetMathLibrary.Normal` (`self.GetVelocity`)) 150.0))) "TraceTypeQuery1"))
  (`self.K2_SetActorRotation` (`KismetMathLibrary.MakeRotFromZX` (`KismetMathLibrary.VInterpTo` (`self.GetActorUpVector`) (`.ImpactNormal` (`GameplayStatics.BreakHitResult` _outhit)) (`GameplayStatics.GetWorldDeltaSeconds`) 10.0) (`self.GetActorForwardVector`)))
  (`CharacterMovementComponent.SetGravityDirection` (`self.CharacterMovement`) (* (`self.GetActorUpVector`) -1.0)))

(fn `SV_Acceleration`
  (params (Forward :type "Float (double-precision)") (Right :type "Float (double-precision)"))
  (set `self.wishdir` (`KismetMathLibrary.Normal` (+ (* Forward (`self.GetActorForwardVector`)) (* Right (`self.GetActorRightVector`)))))
  (set `self.currentspeed` (`KismetMathLibrary.Dot_VectorVector` (`self.GetVelocity`) (`self.wishdir`)))
  (set `self.add speed` (- (`self.SV_Wishspeed`) (`self.currentspeed`)))
  (if (> (`self.add speed`) 0.0)
    (set `self.accelspeed` (* (`self.SV_accelconstant`) (`self.SV_Wishspeed`) (`GameplayStatics.GetWorldDeltaSeconds`)))
    (if (> (`self.accelspeed`) (`self.add speed`))
      (set `self.accelspeed` (`self.add speed`)))
    (`self.AddMovementInput` (`self.wishdir`) (`self.accelspeed`))
    (set `self.Movement_Velocity` (+ (* (`self.wishdir`) (`self.accelspeed`)) (`self.Movement_Velocity`)))))

(fn `SV_AirAccelerate`
  (params (Forward :type "Float (double-precision)") (Right :type "Float (double-precision)"))
  (set `self.wishdir` (`KismetMathLibrary.Normal` (+ (* Forward (`self.GetActorForwardVector`)) (* Right (`self.GetActorRightVector`)))))
  (set `self.AWS` (`self.SV_Wishspeed`))
  (if (> (`self.AWS`) (`self.SV_Air_Accelerating`))
    (set `self.AWS` (`self.SV_Air_Accelerating`)))
  (set `self.currentspeed` (`KismetMathLibrary.Dot_VectorVector` (`self.wishdir`) (`self.GetVelocity`)))
  (set `self.add speed` (- (`self.AWS`) (`self.currentspeed`)))
  (if (> (`self.add speed`) 0.0)
    (set `self.accelspeed` (* (`self.SV_accelconstant`) (`self.SV_Wishspeed`) (`GameplayStatics.GetWorldDeltaSeconds`)))
    (if (> (`self.accelspeed`) (`self.add speed`))
      (set `self.accelspeed` (`self.add speed`)))
    (`self.AddMovementInput` (`self.wishdir`) (`self.accelspeed`))
    (set `self.Movement_Velocity` (+ (* (`self.wishdir`) (`self.accelspeed`)) (`self.Movement_Velocity`)))))

(fn `UserConstructionScript`)